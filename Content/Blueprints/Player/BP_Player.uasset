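; BP_Player is the player Blueprint that places fire, tree or water actors in the world at the mouse cursor.
; On left click it traces under the cursor against static, dynamic and physics-body objects and spawns at the hit location.
; A chain of string comparisons on PlayersSelection picks BP_Fire, BP_Tree or BP_Water.
; PlayersSelection is only read in this graph, never set.
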(event `Key|LeftMouseButton`
  (params (Key :type "Key Structure"))
  (bind (_hitresult _returnvalue) (`PlayerController.GetHitResultUnderCursorForObjects` (`GameplayStatics.GetPlayerController` 0) (`|MakeArray` "ObjectTypeQuery1" "ObjectTypeQuery2" "ObjectTypeQuery4" :!type "EObjectTypeQuery Enum") true))
  (bind (_bblockinghit _binitialoverlap _time _distance _location) (`GameplayStatics.BreakHitResult` _hitresult))
  (bind _returnvalue_2 (`KismetMathLibrary.Conv_VectorToTransform` _location))
  (:`Pressed`
    (if _returnvalue
      (if (`KismetStringLibrary.EqualEqual_StrStr` (`self.PlayersSelection`) "Fire")
        (`|SpawnActorFromClass` "/Game/Blueprints/Fire/BP_Fire.BP_Fire_C" (`KismetMathLibrary.Conv_VectorToTransform` _location) "Undefined" "OverrideRootScale" null null)
        (elif (`KismetStringLibrary.EqualEqual_StrStr` (`self.PlayersSelection`) "Tree")
          (`|SpawnActorFromClass` "/Game/Blueprints/Tree/BP_Tree.BP_Tree_C" _returnvalue_2 "Undefined" "OverrideRootScale" null null)
          (elif (`KismetStringLibrary.EqualEqual_StrStr` (`self.PlayersSelection`) "Water")
            (`|SpawnActorFromClass` "/Game/Blueprints/Water/BP_Water.BP_Water_C" _returnvalue_2 "Undefined" "OverrideRootScale" null null)))))))

(fn `UserConstructionScript`)